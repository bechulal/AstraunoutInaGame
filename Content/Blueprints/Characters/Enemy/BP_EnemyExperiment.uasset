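; Experimental side-view enemy with wall and ledge turning, player detection and an unfinished follow and attack.
; Wall and ground sensor overlaps reverse MoveDirection for EnemyMovement and call Turn, which mirrors the sprite by X scale.
; Detecting the hero records its side and starts a looping timer calling MoveToplayer, which sets location using an offset hero position.
; Timeline-based following and attack animation logic are disconnected, and AttackPlayer is an empty stub.
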(event `self.ReceiveBeginPlay`
  (`KismetSystemLibrary.K2_SetTimerDelegate` (`|CreateDelegate` :!event `EnemyMovement`) 0.01 true))

(event `self.WallDetectionL.OnComponentBeginOverlap`
  (params (OverlappedComponent :type "PrimitiveComponent Object Reference") (OtherActor :type "Actor Object Reference") (OtherComp :type "PrimitiveComponent Object Reference") (OtherBodyIndex :type Integer) (bFromSweep :type Boolean) (SweepResult :type "HitResult Structure (by ref)"))
  ; Left and Right Turning System
  (set `self.OverlappedWallL` true)
  (`self.Turn`)
  (set `self.MoveDirection` (* (`self.MoveDirection`) -1.0)))

(event `self.WallDetectionR.OnComponentBeginOverlap`
  (params (OverlappedComponent :type "PrimitiveComponent Object Reference") (OtherActor :type "Actor Object Reference") (OtherComp :type "PrimitiveComponent Object Reference") (OtherBodyIndex :type Integer) (bFromSweep :type Boolean) (SweepResult :type "HitResult Structure (by ref)"))
  ; Left and Right Turning System
  (set `self.OverlappedWallR` true)
  (`self.Turn`)
  (set `self.MoveDirection` (* (`self.MoveDirection`) -1.0)))

(event `self.GroundDetectionL.OnComponentEndOverlap`
  (params (OverlappedComponent :type "PrimitiveComponent Object Reference") (OtherActor :type "Actor Object Reference") (OtherComp :type "PrimitiveComponent Object Reference") (OtherBodyIndex :type Integer))
  ; Left and Right Turning System
  (set `self.OverlappedGroundL` true)
  (`self.Turn`)
  (set `self.MoveDirection` (* (`self.MoveDirection`) -1.0)))

(event `self.GroundDetectionR.OnComponentEndOverlap`
  (params (OverlappedComponent :type "PrimitiveComponent Object Reference") (OtherActor :type "Actor Object Reference") (OtherComp :type "PrimitiveComponent Object Reference") (OtherBodyIndex :type Integer))
  ; Left and Right Turning System
  (set `self.OverlappedGroundR` true)
  (`self.Turn`)
  (set `self.MoveDirection` (* (`self.MoveDirection`) -1.0)))

(event `self.EnemyDetection.OnComponentBeginOverlap`
  (params (OverlappedComponent :type "PrimitiveComponent Object Reference") (OtherActor :type "Actor Object Reference") (OtherComp :type "PrimitiveComponent Object Reference") (OtherBodyIndex :type Integer) (bFromSweep :type Boolean) (SweepResult :type "HitResult Structure (by ref)"))
  (bind _returnvalue_x (`KismetMathLibrary.BreakVector` (`self.K2_GetActorLocation`)))
  ; Player Detection/Follow/Attack
  (bind _hero_ref (message `/Game/Blueprints/Interfaces/BPI_Interactions.Hero_Ref` OtherActor))
  (`/Engine/EditorBlueprintResources/StandardMacros.IsValid` _hero_ref
    (:`Is Valid`
      (bind _output_get (set `self.Hero Ref` _hero_ref))
      (set `self.SeenPlayer?` true)
      (bind _returnvalue_x_2 (`KismetMathLibrary.BreakVector` (`self.K2_GetActorLocation` _output_get)))
      (`/Engine/EditorBlueprintResources/StandardMacros.CompareFloat` _returnvalue_x_2 _returnvalue_x
        (:`>`
          (set `self.HeroOnRight` true))
        (:`<`
          (set `self.HeroOnLeft` true)))
      (`KismetSystemLibrary.K2_SetTimerDelegate` (delegate `MoveToplayer`) 0.1 true))))

(event `MoveToplayer`
  (bind (_returnvalue_x _returnvalue_y _returnvalue_z) (`KismetMathLibrary.BreakVector` (`self.K2_GetActorLocation` (`self.Hero Ref`))))
  ; Player Detection/Follow/Attack
  (if (`self.SeenPlayer?`)
    (`self.Turn`)
    (`self.K2_SetActorLocation` (`KismetMathLibrary.VLerp` (`self.K2_GetActorLocation`) (`KismetMathLibrary.MakeVector` (- _returnvalue_x 3000.0) _returnvalue_y _returnvalue_z)))))

(event `self.EnemyDetection.OnComponentEndOverlap`
  (params (OverlappedComponent :type "PrimitiveComponent Object Reference") (OtherActor :type "Actor Object Reference") (OtherComp :type "PrimitiveComponent Object Reference") (OtherBodyIndex :type Integer))
  ; Player Detection/Follow/Attack
  (bind _hero_ref (message `/Game/Blueprints/Interfaces/BPI_Interactions.Hero_Ref` OtherActor))
  (`/Engine/EditorBlueprintResources/StandardMacros.IsValid` _hero_ref
    (:`Is Valid`
      (set `self.SeenPlayer?` false)
      (set `self.HeroOnRight` false)
      (set `self.HeroOnLeft` false)
      (`KismetSystemLibrary.K2_SetTimerDelegate` (`|CreateDelegate` :!event `EnemyMovement`) 0.01 true))))

(event `following playr`
  ; Player Detection/Follow/Attack
)

(event `AttackPlayer`
  ; Player Detection/Follow/Attack
)

(fn `EnemyMovement`
  (if (and (not (`self.IsAttacking?`)) (not (`self.AtPlayerLoc`)))
    (`self.AddMovementInput` (`KismetMathLibrary.Vector_Forward`) (`self.MoveDirection`))))

(fn `Turn`
  (if (`self.HeroOnLeft`)
    (`SceneComponent.SetRelativeScale3D` (`self.Sprite`) (-0.374089 0.374089 0.374089))
    (elif (`self.HeroOnRight`)
      (`SceneComponent.SetRelativeScale3D` (`self.Sprite`) (0.374089 0.374089 0.374089))
      (elif (`self.OverlappedWallR`)
        (`SceneComponent.SetRelativeScale3D` (`self.Sprite`) (-0.374089 0.374089 0.374089))
        (set `self.OverlappedWallR` false)
        (elif (`self.OverlappedWallL`)
          (`SceneComponent.SetRelativeScale3D` (`self.Sprite`) (0.374089 0.374089 0.374089))
          (set `self.OverlappedWallL` false)
          (elif (`self.OverlappedGroundR`)
            (`SceneComponent.SetRelativeScale3D` (`self.Sprite`) (-0.374089 0.374089 0.374089))
            (set `self.OverlappedGroundR` false)
            (elif (`self.OverlappedGroundL`)
              (`SceneComponent.SetRelativeScale3D` (`self.Sprite`) (0.374089 0.374089 0.374089))
              (set `self.OverlappedGroundL` false))))))))

(fn `UserConstructionScript`)