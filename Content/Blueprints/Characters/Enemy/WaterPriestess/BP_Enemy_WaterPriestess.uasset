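; Water Priestess enemy Blueprint for a scripted villain defeat tied to dialogue.
; On BeginPlay it unpossesses its AI controller and binds KillTheVillain to the dialogue box's finished event.
; KillTheVillain jumps the animation to its defeated node and flickers the sprite on a looping timer.
; After a short delay it stops the flicker, destroys the actor and calls the ECallDialogue5 dispatcher.
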(event `self.ReceiveBeginPlay`
  (`parent.ReceiveBeginPlay`)
  (bind _asaicontroller (cast `AIController` (`self.GetController`)))
  (`Controller.UnPossess` _asaicontroller)
  (add `/Game/Blueprints/BP_DialogueBox4.E_OnDialogueFinished` (`self.DialogueBoxRef`) (delegate `KillTheVillain`)))

(event `KillTheVillain`
  (`KismetSystemLibrary.PrintString` "Hello")
  (`PaperZDAnimInstance.JumpToNode` (`self.AnimInstance`) "JumpDefeated" "None")
  (bind _returnvalue (`KismetSystemLibrary.K2_SetTimerDelegate` (`|CreateDelegate` :!event `StartSpriteFlicker`) 0.04 true))
  (set `self.TimerHandle` _returnvalue)
  (`KismetSystemLibrary.Delay` 2.0)
  (`self.StopSpriteFlicker`)
  (`self.K2_DestroyActor`)
  (`self.E_CallDialogue5`))

(fn `StartSpriteFlicker`
  (`SceneComponent.SetVisibility` (`self.Sprite`) (not (`SceneComponent.bVisible` (`self.Sprite`))) false))

(fn `StopSpriteFlicker`
  (`KismetSystemLibrary.K2_ClearAndInvalidateTimerHandle` (`self.TimerHandle`))
  (`SceneComponent.SetVisibility` (`self.Sprite`) false false))

(fn `UserConstructionScript`
  (`parent.UserConstructionScript`))