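; BP_PatrolTrack is a spline-based patrol route for enemy AI.
; It tracks a current index into the points of its PatrolTrack spline and returns that point's world location through GetSplineWorldLoc.
; IncrementPatrolRoute steps the index and reverses direction at the first and last points, so the route runs back and forth instead of looping.
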(event `IncrementPatrolRoute`
  (set `self.PatrolIndex` (+ (`self.PatrolIndex`) (`self.DIrection`)))
  (if (== (`self.PatrolIndex`) (- (`SplineComponent.GetNumberOfSplinePoints` (`self.PatrolTrack`)) 1))
    (set `self.DIrection` -1)
    (elif (== (`self.PatrolIndex`) 0)
      (set `self.DIrection` 1))))

(fn `GetSplineWorldLoc`
  (returns (SplineWorldLoc :type "Vector Structure"))
  (return (`SplineComponent.GetLocationAtSplinePoint` (`self.PatrolTrack`) (`self.PatrolIndex`) "World")))

(fn `UserConstructionScript`)