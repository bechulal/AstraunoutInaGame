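; Goblin enemy Blueprint that configures inherited enemy behavior with goblin-specific attack, death sound and damage.
; BeginPlay runs the parent logic first, then assigns the attack animation, death sound cue and damage value.
; ChangingAnimation is an empty stub, and the construction script only calls the parent.
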(event `self.ReceiveBeginPlay`
  (`parent.ReceiveBeginPlay`)
  (set `self.AttackAnimation` "/Game/Blueprints/Characters/Enemy/Goblin/AnimSequences/Attack.Attack")
  (set `self.DeathSound` "/Game/Blueprints/Characters/Enemy/Goblin/goblin-death_Cue.goblin-death_Cue")
  (set `self.Damage` 25.0))

(fn `ChangingAnimation`
  (returns (Animation :type "PaperZDAnimationComponent Object Reference")))

(fn `UserConstructionScript`
  (`parent.UserConstructionScript`))