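; Player-controlled Paper2D astronaut character that runs left and right and jumps, using Enhanced Input.
; Movement, jump and fall state pick gun-carrying flipbooks through FSetMovementAnimation, which turns the sprite to face the run direction.
; Coyote time grants a Status.CanJump gameplay tag briefly on falling without upward velocity, letting jump input launch the character upward.
; A looping timer started on jump or airborne movement switches to fall and idle animations.
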(event `self.ReceiveBeginPlay`
  (bind _asplayer_controller (cast `PlayerController` (`self.GetController`)))
  (`EnhancedInputSubsystemInterface.AddMappingContext` (pcsubsystem `EnhancedInputLocalPlayerSubsystem` _asplayer_controller) "/Game/Blueprints/Characters/Astranaut/Input/IMC_Astranaut.IMC_Astranaut" 0 (struct)))

(event `EnhancedInput|/Game/Blueprints/Characters/Astranaut/Input/IA_Move`
  (params (ActionValue :type "Float (double-precision)") (ElapsedSeconds :type "Float (double-precision)") (TriggeredSeconds :type "Float (double-precision)") (InputAction :type "InputAction Object Reference" :default "/Game/Blueprints/Characters/Astranaut/Input/IA_Move.IA_Move"))
  ; Movement
  (:`Triggered`
    (set `self.MovementActionValue` ActionValue)
    (`self.AddMovementInput` (`self.GetActorForwardVector`) ActionValue)
    (if (`NavMovementInterface.IsFalling` (`self.CharacterMovement`))
      (`self.f_SetMovementAnimation` "NewEnumerator4")
      (`self.CheckIsFalling`)
      (elif (> ActionValue 0.0)
        (`self.f_SetMovementAnimation` "NewEnumerator1")
        (elif (< ActionValue 0.0)
          (`self.f_SetMovementAnimation` "NewEnumerator2")
          (else
            (`self.f_SetMovementAnimation` "NewEnumerator0"))))))
  (:`Completed`
    (set `self.MovementActionValue` 0.0)
    (if (not (`NavMovementInterface.IsFalling` (`self.CharacterMovement`)))
      (`self.f_SetMovementAnimation` "NewEnumerator0"))))

(event `EnhancedInput|/Game/Blueprints/Characters/Astranaut/Input/IA_Jump`
  (params (ActionValue :type Boolean) (ElapsedSeconds :type "Float (double-precision)") (TriggeredSeconds :type "Float (double-precision)") (InputAction :type "InputAction Object Reference" :default "/Game/Blueprints/Characters/Astranaut/Input/IA_Jump.IA_Jump"))
  ; Implementing Jump and Coyote Time
  (:`Started`
    (`self.Jump`)
    (`self.f_SetMovementAnimation` "NewEnumerator4")
    (`self.CheckIsFalling`)
    (if (`BlueprintGameplayTagLibrary.HasTag` (`self.GamePlayTags`) (struct :`TagName` "Status.CanJump?") true)
      (`self.LaunchCharacter` (0.0 0.0 400.0))))
  (:`Canceled`
    (if (not (`NavMovementInterface.IsFalling` (`self.CharacterMovement`)))
      (`self.StopJumping`))))

(event `self.K2_OnMovementModeChanged`
  (params (PrevMovementMode :type "EMovementMode Enum" :default "MOVE_None") (NewMovementMode :type "EMovementMode Enum" :default "MOVE_None") (PrevCustomMode :type Byte) (NewCustomMode :type Byte))
  (bind (_velocity_x _velocity_y _velocity_z) (`KismetMathLibrary.BreakVector` (`MovementComponent.Velocity` (`self.CharacterMovement`))))
  ; Implementing Jump and Coyote Time
  (if (`|EnumEquality` NewMovementMode "MOVE_Falling")
    (if (<= _velocity_z 0.0)
      (`BlueprintGameplayTagLibrary.AddGameplayTag` (`self.GamePlayTags`) (struct :`TagName` "Status.CanJump?"))
      (`KismetSystemLibrary.RetriggerableDelay` 0.2)
      (`BlueprintGameplayTagLibrary.RemoveGameplayTag` (`self.GamePlayTags`) (struct :`TagName` "Status.CanJump?"))
      (else
        (`BlueprintGameplayTagLibrary.RemoveGameplayTag` (`self.GamePlayTags`) (struct :`TagName` "Status.CanJump?"))))))

(event `CheckIsFalling`
  (bind _returnvalue (`KismetSystemLibrary.K2_SetTimerDelegate` (delegate `CheckIsFallingLoop`) 0.05 true))
  (set `self.CheckIfFallingTimer` _returnvalue))

(event `CheckIsFallingLoop`
  (if (`NavMovementInterface.IsFalling` (`self.CharacterMovement`))
    (`KismetSystemLibrary.Delay` 0.3)
    (`self.f_SetMovementAnimation` "NewEnumerator5")
    (if (`NavMovementInterface.IsFalling` (`self.CharacterMovement`))
      _
      (elif (== (`self.MovementActionValue`) 0.0)
        (`self.f_SetMovementAnimation` "NewEnumerator0")))
    (else
      (`self.f_SetMovementAnimation` "NewEnumerator0")
      (`KismetSystemLibrary.K2_ClearAndInvalidateTimerHandle` (`self.CheckIfFallingTimer`)))))

(fn `f_SetMovementAnimation`
  (params (MovementEnum :type "/Game/Blueprints/Characters/Astranaut/Enums/E_MovementStates Enum" :default "NewEnumerator0"))
  (bind _sprite (`self.Sprite`))
  (`PaperFlipbookComponent.SetLooping` (`self.Sprite`) (select `/Game/Blueprints/Characters/Astranaut/Enums/E_MovementStates` MovementEnum :`NewEnumerator0` true :`NewEnumerator1` true :`NewEnumerator2` true))
  (`PaperFlipbookComponent.Play` (`self.Sprite`))
  (switch `/Game/Blueprints/Characters/Astranaut/Enums/E_MovementStates` MovementEnum
    (:`NewEnumerator0`
      (`PaperFlipbookComponent.SetFlipbook` _sprite "/Game/Assets/Astranaut/player__Idle_gun.player__Idle_gun"))
    (:`NewEnumerator1`
      (`PaperFlipbookComponent.SetFlipbook` _sprite "/Game/Assets/Astranaut/player__Run_with_Gun.player__Run_with_Gun")
      (`SceneComponent.K2_SetRelativeRotation` :`self` (`self.Sprite`)))
    (:`NewEnumerator2`
      (`PaperFlipbookComponent.SetFlipbook` _sprite "/Game/Assets/Astranaut/player__Run_with_Gun.player__Run_with_Gun")
      (`SceneComponent.K2_SetRelativeRotation` (`self.Sprite`) (struct :`Yaw` -180.0) false false))
    (:`NewEnumerator4`
      (`PaperFlipbookComponent.SetFlipbook` _sprite "/Game/Assets/Astranaut/player__JumpGunRise.player__JumpGunRise"))
    (:`NewEnumerator5`
      (`PaperFlipbookComponent.SetFlipbook` _sprite "/Game/Assets/Astranaut/player__JumpGunFall.player__JumpGunFall"))))

(fn `UserConstructionScript`)