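; BP_DialogueBox4 is a dialogue trigger that advances through its text lines, one per valid hero overlap.
; An interface message identifies the hero, then a lazily created WBP_Dialogue widget displays the indexed line.
; Once the index exceeds the array length, it hides the widget and broadcasts a dialogue-finished event.
; The DialogueBox3Ref function enables the trigger's query collision, while the other interface-style functions are empty stubs.
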(event `self.ReceiveBeginPlay`)

(event `self.DialogueTrigger.OnComponentBeginOverlap`
  (params (OverlappedComponent :type "PrimitiveComponent Object Reference") (OtherActor :type "Actor Object Reference") (OtherComp :type "PrimitiveComponent Object Reference") (OtherBodyIndex :type Integer) (bFromSweep :type Boolean) (SweepResult :type "HitResult Structure (by ref)"))
  (bind _hero_ref (message `/Game/Blueprints/Interfaces/BPI_Interactions.Hero_Ref` OtherActor))
  (`/Engine/EditorBlueprintResources/StandardMacros.IsValid` _hero_ref
    (:`Is Valid`
      (`/Engine/EditorBlueprintResources/StandardMacros.IncrementInt` (`self.DialogueIndex`)
        (:`  `
          (if (<= (`self.DialogueIndex`) (`KismetArrayLibrary.Array_Length` (`self.DialogueLines`)))
            (`self.DialogueUI`
              (:`then`
                _)
              (:`else`
                (bind _returnvalue (`|CreateWidget` "/Game/Blueprints/WBP_Dialogue.WBP_Dialogue_C"))
                (set `self.DialogueUI` _returnvalue)
                (`UserWidget.AddToViewport` _returnvalue 0)))
            (`TextBlock.SetText` (`/Game/Blueprints/WBP_Dialogue.DialogueText` (`self.DialogueUI`)) (`|GetArrayItem` (`self.DialogueLines`) (`self.DialogueIndex`)))
            (else
              (`Widget.SetVisibility` (`self.DialogueUI`) "Hidden")
              (`self.E_OnDialogueFinished`))))))
    (:`Is Not Valid`
      (`KismetSystemLibrary.PrintString` "Not valid"))))

(event `self.DialogueTrigger.OnComponentEndOverlap`
  (params (OverlappedComponent :type "PrimitiveComponent Object Reference") (OtherActor :type "Actor Object Reference") (OtherComp :type "PrimitiveComponent Object Reference") (OtherBodyIndex :type Integer)))

(fn `ChangingAnimation`
  (returns (Animation :type "PaperZDAnimationComponent Object Reference"))
  (return null))

(fn `DialogueBox3_Ref`
  (`PrimitiveComponent.SetCollisionEnabled` (`self.DialogueTrigger`) "QueryOnly")
  (return))

(fn `Enemy_Ref`
  (returns (Enemy_Ref :type "/Game/Blueprints/Characters/Enemy/BP_Enemy Object Reference"))
  (return null))

(fn `FirstLevelRef`
  (returns (ref :type "Actor Object Reference"))
  (return null))

(fn `Hero_Ref`
  (returns (Hero_Ref :type "/Game/Blueprints/Characters/FireHero/BP_FireHero Object Reference"))
  (return null))

(fn `Interact`
  (return))

(fn `MovementSpeed`
  (params (Speed :type "/Game/Blueprints/Characters/Enemy/Enums/E_Enemy_Speed Enum" :default "NewEnumerator0"))
  (returns (SpeedValue :type "Float (double-precision)"))
  (return 0.0))

(fn `SplinePointRef`
  (returns (SplinePointRef :type "/Game/Blueprints/Characters/Enemy/AI/BP_PatrolTrack Object Reference"))
  (return null))

(fn `UserConstructionScript`)